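; Player-controlled tank pawn Blueprint that binds input to driving, camera aiming and firing.
; Aim axes rotate the azimuth gimbal (yaw) and spring arm (pitch), scaled by frame delta time.
; Throttle and move axes pass intents to the TankMovement component, and the Fire action calls Fire.
; BeginPlay hands barrel and turret references to the tank and both tracks to TankMovement.
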(event `InputAxis|AimAzimuth`
  (params (AxisValue :type "Float (single-precision)"))
  ;[1 1 1] Input binding
  (`SceneComponent.K2_AddLocalRotation` (`self.Azimuth Gimbal`) (`KismetMathLibrary.MakeRotator` 0.0 0.0 (* AxisValue (`GameplayStatics.GetWorldDeltaSeconds`) 100.0)) false false))

(event `InputAxis|Left Track Throttle`
  (params (AxisValue :type "Float (single-precision)"))
  (`TankMovementComponent.intendTurnLeft` (`self.TankMovement`) AxisValue))

(event `InputAxis|AimElevation`
  (params (AxisValue :type "Float (single-precision)"))
  ;[1 1 1] Input binding
  (`SceneComponent.K2_AddLocalRotation` (`self.SpringArm`) (`KismetMathLibrary.MakeRotator` 0.0 (* AxisValue (`GameplayStatics.GetWorldDeltaSeconds`) 100.0)) false false))

(event `InputAxis|Right Track Throttle`
  (params (AxisValue :type "Float (single-precision)"))
  (`TankMovementComponent.intendTurnRight` (`self.TankMovement`) AxisValue))

(event `InputAction|Fire`
  (params (Key :type "Key Structure" :default "AnyKey"))
  ;[1 1 1] Input binding
  (:`Pressed`
    (`self.Fire`)))

(event `InputAxis|Move Backward`
  (params (AxisValue :type "Float (single-precision)"))
  (`TankMovementComponent.intendMoveForward` (`self.TankMovement`) AxisValue))

(event `InputAxis|Move Forward`
  (params (AxisValue :type "Float (single-precision)"))
  (`TankMovementComponent.intendMoveForward` (`self.TankMovement`) AxisValue))

(event `self.ReceiveBeginPlay`
  (`self.SetBarrelReference` (`self.TankBarrel`))
  (`self.SetTurretReference` (`self.TankTurret`))
  (`TankMovementComponent.setTracksReference` (`self.TankMovement`) (`self.TankRightTrack`) (`self.TankLeftTrack`)))

(fn `UserConstructionScript`)